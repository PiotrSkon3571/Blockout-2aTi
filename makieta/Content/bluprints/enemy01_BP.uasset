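; Enemy pawn Blueprint that continually chases the first player character.
; On BeginPlay it runs AI MoveTo toward the player, then restarts the move after a short delay whether it succeeds or fails.
; When the player overlaps its Box1 trigger, a set of cube and other components switch to a new material.
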(event OnComponentBeginOverlap(Box1)
  (params (OverlappedComponent :type Primitive%20Component%20Object%20Reference) (OtherActor :type Actor%20Object%20Reference) (OtherComp :type Primitive%20Component%20Object%20Reference) (OtherBodyIndex :type Integer) (bFromSweep :type Boolean) (SweepResult :type Hit%20Result%20Structure%20%28by%20ref%29))
  (if (== (Game|GetPlayerCharacter 0) OtherActor)
    (Rendering|Material|SetMaterial (Variables|Default|GetCube) 0 "/Game/ThirdPersonBP/textury/trees/NewMaterial1.NewMaterial1")))

(event EventBeginPlay
  (AI|AIMoveTo self "0.000000,300.000000,0.000000" (Game|GetPlayerCharacter 0) 5.0 false :!label _label
    (:OnSuccess
      _)
    (:OnFail
      _))
  (Utilities|FlowControl|Delay 0.2)
  (goto _label))

(fn ConstructionScript)